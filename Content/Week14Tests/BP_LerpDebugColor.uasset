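; BP_LerpDebugColor is a test actor that visualizes HSV color interpolation with temporary debug spheres.
; On BeginPlay a loop draws 100 spheres at the actor's X, cycling world Y every ten while height climbs each iteration.
; The same accumulating Step drives height and the orange-to-blue lerp alpha, which grows past 1 without clamping.
; An unconnected Timeline version of the lerp exercise never runs.
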(event EventBeginPlay
  (bind _returnvalue (Transformation|GetActorLocation))
  (for _index (range 0 99)
    (Rendering|Debug|DrawDebugSphere (Math|Vector|MakeVector (.x _returnvalue) (* (Math|Conversions|ToFloat(Integer) (Math|Integer|%(Integer) _index 10)) 1.5e+02) (+ (.z _returnvalue) (* (Variables|Default|GetStep) 1.5e+03))) 1e+02 24 (Class|KismetMathLibrary|LinearColorLerpUsingHSV "(R=1.000000,G=0.359390,B=0.000000,A=1.000000)" "(R=0.000000,G=0.675589,B=1.000000,A=1.000000)" (Variables|Default|GetStep)) 12.0 4.0)
    (Variables|Default|SetStep (+ (Variables|Default|GetStep) 0.1))))

(fn ConstructionScript)