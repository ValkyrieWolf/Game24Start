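; BP_Weapon is a weapon Blueprint with randomized damage and text displays for weapon type, elemental type and damage range.
; RandomizeValues rolls minimum and maximum damage, then calls UpdateText to refresh the labels.
; UpdateText also registers the weapon in the GM_LevelSawp game mode's LevelSave spawned-weapon list, and skips both steps if that cast fails.
; LoadSpawnedState only prints a message.
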(event Custom|LoadSpawnedState
  (Development|PrintString "Get Your Weapons HERE!" true true "(R=1.000000,G=0.000000,B=0.071003,A=1.000000)"))

(event Custom|Randomize%20Values
  (bind _output_get (Variables|Default|SetMinDamage (+ (Variables|Default|GetMinDamage) (Math|Random|RandomInteger 2))))
  (Variables|Default|SetMaxDamage (+ _output_get (Math|Random|RandomInteger 4)))
  (CallFunction|UpdateText))

(event Custom|Update%20Text
  (bind _asgm_level_sawp (Utilities|Casting|CastToGM_LevelSawp (Game|GetGameMode)))
  (Utilities|Array|AddUnique (Variables|/Game/Blueprints/Saving_Loading/SG_SaveLevel.SG_SaveLevel_C|GetSpawnedWeapon (Variables|/Game/Blueprints/Saving_Loading/GM_LevelSawp.GM_LevelSawp_C|GetLevel%20Save _asgm_level_sawp)) self)
  (Rendering|Components|TextRender|SetText (Variables|Default|GetTextWeaponType) (Utilities|Text|ToText(String) (Utilities|String|EnumtoString (Variables|Default|GetWeaponType))))
  (Rendering|Components|TextRender|SetText (Variables|Default|GetDamageType) (Utilities|Text|ToText(String) (Utilities|String|EnumtoString (Variables|Default|GetElementalType))))
  (Rendering|Components|TextRender|SetText (Variables|Default|GetDamage) (Utilities|Text|ToText(String) (Utilities|String|Append (Utilities|String|ToString(Integer) (Variables|Default|GetMinDamage)) "-" (Utilities|String|ToString(Integer) (Variables|Default|GetMaxDamage))))))

(fn ConstructionScript)