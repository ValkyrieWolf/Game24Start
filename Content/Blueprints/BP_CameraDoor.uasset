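; BP_CameraDoor is a door actor that briefly becomes the view target to show itself opening.
; OpenDoor, gated by Closed, records the door in the game mode's LevelSave, blends the requesting player's camera to it, then lowers the Door component by Timeline.
; After a pause it blends player controller 0 to the supplied view target.
; quietOpen plays the same motion without camera or save steps; both paths end setting Closed true.
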(event Custom|OpenDoor
  (params (NewViewTarget :type Actor%20Object%20Reference) (PlayerIndex :type Integer))
  (if (Variables|Default|GetClosed)
    (bind _asgm_level_sawp (Utilities|Casting|CastToGM_LevelSawp (Game|GetGameMode)))
    (Utilities|Array|AddUnique (Variables|/Game/Blueprints/Saving_Loading/SG_SaveLevel.SG_SaveLevel_C|GetOpenDoors (Variables|/Game/Blueprints/Saving_Loading/GM_LevelSawp.GM_LevelSawp_C|GetLevel%20Save _asgm_level_sawp)) self)
    (Game|Player|SetViewTargetwithBlend (Class|GameplayStatics|GetPlayerControllerfromID PlayerIndex) self (Variables|Default|GetBlend%20Time) "VTBlend_Cubic" 0.0 true)
    (Utilities|FlowControl|Delay (Variables|Default|GetBlend%20Time))
    (bind _newtrack_0 (Timeline|Timeline Play)
      (:Update
        (Transformation|SetRelativeLocation (Variables|Default|GetDoor) (Math|Vector|Lerp(Vector) "0.000000,0.000000,150.000000" "0.000000,0.000000,-130.000000" _newtrack_0) false false))
      (:Finished
        (Utilities|FlowControl|Delay 2.0) ; waiting 2 seconds while the door opens
        (Game|Player|SetViewTargetwithBlend (Game|GetPlayerController 0) NewViewTarget (/ (Variables|Default|GetBlend%20Time) 2.0) "VTBlend_Cubic" 0.0 false) ; shift camera back to player
        (Variables|Default|SetClosed true)))))

(event Custom|quietOpen
  (bind _newtrack_0 (Timeline|Timeline_0 Play)
    (:Update
      (Transformation|SetRelativeLocation (Variables|Default|GetDoor) (Math|Vector|Lerp(Vector) "0.000000,0.000000,150.000000" "0.000000,0.000000,-130.000000" _newtrack_0) false false))
    (:Finished
      (Variables|Default|SetClosed true))))

(fn ConstructionScript)