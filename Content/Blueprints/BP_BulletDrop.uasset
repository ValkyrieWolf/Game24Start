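; Bullet drop test Blueprint that draws a hand-calculated projectile arc from its Arrow beside the engine's predicted path for comparison.
; Every 1.2 seconds, ReallyCoolBulletDropCalc steps through the simulation with debug lines, spheres and line traces, stopping on a hit, then resets.
; Each step divides only X velocity by SimFrequency and adds gravity to Z scaled by its square.
; PredictProjectilePath Advanced then traces from the same Arrow using StartingVelocity.
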(event Custom|Really%20Cool%20Bullet%20Drop%20Calc
  (bind _maxsimtime (Variables|Default|GetMaxSimTime))
  (Variables|Default|SetEnd (+ (Variables|Default|GetStart%20Location) (/ (Variables|Default|GetVelocity) (Math|Vector|MakeVector (Variables|Default|GetSim%20Frequency) 1.0 1.0))))
  (Utilities|FlowControl|ForLoopwithBreak 0 (- (Math|Float|Truncate (* (Variables|Default|GetMaxSimTime) (Variables|Default|GetSim%20Frequency))) 1) :!label _label
    (:LoopBody
      (Rendering|Debug|DrawDebugLine (Variables|Default|GetStart%20Location) (+ (Variables|Default|GetStart%20Location) (/ (Variables|Default|GetVelocity) (Math|Vector|MakeVector (Variables|Default|GetSim%20Frequency) 1.0 1.0))) "(R=0.000000,G=1.000000,B=0.956688,A=1.000000)" _maxsimtime 0.0)
      (Rendering|Debug|DrawDebugSphere (+ (Variables|Default|GetStart%20Location) (/ (Variables|Default|GetVelocity) (Math|Vector|MakeVector (Variables|Default|GetSim%20Frequency) 1.0 1.0))) 5.0 12 "(R=0.000000,G=0.122433,B=1.000000,A=1.000000)" _maxsimtime)
      (bind _returnvalue (Class|KismetSystemLibrary|LineTraceSinglebyProfile (Variables|Default|GetStart%20Location) (Variables|Default|GetEnd) "BlockAll" false 0 "None" true))
      (if _returnvalue
        (Development|PrintString "Hit Something" true true "(R=1.000000,G=0.000000,B=0.953886,A=1.000000)")
        (goto _label Break)
        (else
          (Variables|Default|SetStart%20Location (Variables|Default|GetEnd)) ; Set the new start location
          (Variables|Default|SetVelocity (+ (Variables|Default|GetVelocity) (Math|Vector|MakeVector 0.0 0.0 (/ -9.8e+02 (Math|Float|Square (Variables|Default|GetSim%20Frequency))))))
          (Variables|Default|SetEnd (+ (Variables|Default|GetStart%20Location) (/ (Variables|Default|GetVelocity) (Math|Vector|MakeVector (Variables|Default|GetSim%20Frequency) 1.0 1.0)))))))
    (:Completed
      (Variables|Default|SetStart%20Location (Transformation|GetWorldLocation (Variables|Default|GetArrow)))
      (Variables|Default|SetVelocity (Variables|Default|GetStartingVelocity)))))

(event EventBeginPlay
  (bind _arrow (Variables|Default|GetArrow))
  (bind _returnvalue (Transformation|GetWorldLocation _arrow))
  (Variables|Default|SetStart%20Location _returnvalue)
  (Utilities|FlowControl|Sequence :!label _label
    (:then_0
      (CallFunction|ReallyCoolBulletDropCalc))
    (:then_1
      (Class|GameplayStatics|BlueprintPredictProjectilePathAdvanced (Utilities|Struct|MakePredictProjectilePathParams _returnvalue (Variables|Default|GetStartingVelocity) true 0.0 (Variables|Default|GetMaxSimTime) true "ECC_WorldStatic" "ObjectTypeQuery1" 0 (Variables|Default|GetSim%20Frequency) 0.0 "ForDuration" 1.0 false))
      (Utilities|FlowControl|Delay 1.2)
      (goto _label))))

(fn ConstructionScript)