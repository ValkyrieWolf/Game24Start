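; Game mode that handles per-level saving and loading, using the current level name as the save slot.
; On BeginPlay it loads the SG_SaveLevel save to restore collected coins, open doors and any non-zero player location, or creates a new one if missing or invalid.
; Checkpoint stores the player transform and saves.
; FinishedLevel clears that transform, saves and calls ResetLevel.
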(event Custom|Save%20Game
  (bind _returnvalue (Game|GetCurrentLevelName true))
  (bind _returnvalue_2 (SaveGame|SaveGametoSlot (Variables|Default|GetLevel%20Save) _returnvalue))
  (if _returnvalue_2
    (Development|PrintString "Saved Level!")
    (else
      (Development|PrintString "warning:COULD NOT SAVE LEVEL" true true "(R=1.000000,G=0.000000,B=0.118507,A=1.000000)"))))

(event EventBeginPlay
  (Development|PrintString "Loaded new Game Mode!" true true "(R=1.000000,G=0.018841,B=0.681485,A=1.000000)" 5.0)
  ;[1 1 1] Is there a level save file for this level's name? If not, create one, so that we can start editing it. If there is - load it and store it to the "Level Save" variable, so we can start editing it.
  (bind _returnvalue (Game|GetCurrentLevelName true))
  (bind _returnvalue_2 (SaveGame|DoesSaveGameExist _returnvalue))
  (if _returnvalue_2
    (bind _returnvalue_3 (SaveGame|LoadGamefromSlot _returnvalue))
    (bind _assg_save_level (Utilities|Casting|CastToSG_SaveLevel _returnvalue_3)
      (:then
        (bind _output_get (Variables|Default|SetLevel%20Save _assg_save_level))
        (Default|LoadCollectedCoins _output_get)
        (Default|LoadOpenDoors _output_get)
        (if (not (Class|KismetMathLibrary|EqualExactlyVectorVector (.location (Variables|/Game/Blueprints/Saving_Loading/SG_SaveLevel.SG_SaveLevel_C|GetPlayerTransform (Variables|Default|GetLevel%20Save))) "0, 0, 0"))
          (Transformation|SetWorldTransform (Variables|/Script/Engine.Character|GetCapsuleComponent (Game|GetPlayerCharacter 0)) (Variables|/Game/Blueprints/Saving_Loading/SG_SaveLevel.SG_SaveLevel_C|GetPlayerTransform (Variables|Default|GetLevel%20Save)) false false)))
      (:CastFailed
        (SaveGame|DeleteGameinSlot _returnvalue)
        (bind _returnvalue_4 (SaveGame|CreateSaveGameObject "/Game/Blueprints/Saving_Loading/SG_SaveLevel.SG_SaveLevel_C" :!label _label))
        (Variables|Default|SetLevel%20Save _returnvalue_4)))
    (else
      (goto _label))))

(fn ConstructionScript)

(fn Checkpoint
  (params (Player%20Transform :type Transform))
  (Variables|/Game/Blueprints/Saving_Loading/SG_SaveLevel.SG_SaveLevel_C|SetPlayerTransform (Variables|Default|GetLevel%20Save) Player%20Transform)
  (CallFunction|SaveGame))

(fn FinishedLevel
  (Variables|/Game/Blueprints/Saving_Loading/SG_SaveLevel.SG_SaveLevel_C|SetPlayerTransform (Variables|Default|GetLevel%20Save) "")
  (CallFunction|SaveGame)
  (Class|GameModeBase|ResetLevel))