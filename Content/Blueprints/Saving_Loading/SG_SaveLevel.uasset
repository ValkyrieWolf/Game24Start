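; SG_SaveLevel holds saved level state for collected coins, open doors, moved blocks and spawned weapons, and reapplies it on load.
; Each category has its own load function that loops over a stored array, skips invalid references and tells each object to restore itself.
; Coins, blocks and weapons call their own load methods, while doors use QuietOpen.
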(fn LoadCollectedCoins
  (if (> (Utilities|Array|Length (Variables|Default|GetCollectedCoins)) 0) ; Do we have any coins that are already collected?
    (for _array_element (Variables|Default|GetCollectedCoins)
      (Utilities|IsValid _array_element
        (:Is%20Valid
          (Default|LoadCollectedState _array_element))))))

(fn LoadOpenDoors
  (bind _opendoors (Variables|Default|GetOpenDoors))
  (if (> (Utilities|Array|Length _opendoors) 0) ; Do we have any coins that are already collected?
    (for _array_element _opendoors
      (Utilities|IsValid _array_element
        (:Is%20Valid
          (Default|QuietOpen _array_element))))))

(fn LoadCubes
  (bind _movedblock (Variables|Default|GetMovedBlock))
  (if (> (Utilities|Array|Length _movedblock) 0)
    (for _array_element _movedblock
      (Utilities|IsValid _array_element
        (:Is%20Valid
          (Default|LoadCubes _array_element))))))

(fn LoadWeapons
  (for _array_element (Variables|Default|GetSpawnedWeapon)
    (Utilities|IsValid _array_element
      (:Is%20Valid
        (Default|LoadSpawnedState _array_element)))))